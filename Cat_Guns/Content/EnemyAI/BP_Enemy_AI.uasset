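; Enemy AI that chases the first-person player and shoots projectiles at them.
; When pawn sensing sees the player, it turns to face them, starts AIMoveTo and fires from BulletSpawner, gated by a CanAttack cooldown.
; TakeDamage decrements Health and, at zero, destroys the enemy and increments the player's KillScore.
; DeactivateEnemy hides it and disables collision, tick and attacks; an ApplyDamage attack chain is left unconnected.
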(event OnSeePawn(PawnSensing)
  (params (Pawn :type Pawn%20Object%20Reference))
  (bind _asbp_first_person_character (Utilities|Casting|CastToBP_FirstPersonCharacter Pawn))
  (Transformation|SetActorRotation (Math|Rotator|FindRelativeLookatRotation (Math|Conversions|ToTransform(Vector) (Transformation|GetActorLocation)) (Transformation|GetActorLocation _asbp_first_person_character)))
  (AI|AIMoveTo self (Transformation|GetActorLocation) _asbp_first_person_character 1e+01 false
    (:then
      (if (Variables|Default|GetcanAttack?)
        (Game|SpawnActorfromClass "/Game/FirstPerson/Blueprints/BP_FirstPersonProjectile.BP_FirstPersonProjectile_C" (Transformation|GetWorldTransform (Variables|Default|GetBullet%20Spawner)) "Undefined" "MultiplyWithRoot" 0 0)
        (Variables|Default|SetcanAttack? false)
        (Utilities|FlowControl|Delay 0.8)
        (Variables|Default|SetcanAttack? true)))))

(event Custom|Take%20Damage
  (Variables|Default|SetHealth (- (Variables|Default|GetHealth) 1))
  (if (<= (Variables|Default|GetHealth) 0)
    (Actor|DestroyActor)
    (Development|PrintString "Dead Enemy")
    (CallFunction|KillScoreUp)))

(event Custom|Deactivate%20Enemy
  (Rendering|SetActorHiddenInGame true)
  (Collision|SetActorEnableCollision false)
  (Actor|Tick|SetActorTickEnabled false)
  (Variables|Default|SetcanAttack? false))

(event Custom|Kill%20Score%20Up
  (bind _asbp_first_person_character (Utilities|Casting|CastToBP_FirstPersonCharacter (Game|GetPlayerCharacter 0)))
  (Variables|/Game/FirstPerson/Blueprints/BP_FirstPersonCharacter.BP_FirstPersonCharacter_C|SetKillScore _asbp_first_person_character (+ (Variables|/Game/FirstPerson/Blueprints/BP_FirstPersonCharacter.BP_FirstPersonCharacter_C|GetKillScore _asbp_first_person_character) 1)))

(event EventBeginPlay)

(event Collision|EventActorBeginOverlap
  (params (OtherActor :type Actor%20Object%20Reference)))

(event EventTick
  (params (DeltaSeconds :type Float%20%28single-precision%29)))

(fn ConstructionScript)